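; AI character that runs the BT_Test behavior tree and tracks the player through AI perception.
; Sensing the third-person character writes it to the PlayerRef blackboard key and cancels the lost-vision timer.
; Losing it starts a two-second timer that clears the key, giving a short memory before the AI forgets.
; An unused random-roam loop and a collectible cast remain disconnected.
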(event OnTargetPerceptionUpdated(AIPerception)
  (params (Actor :type Actor%20Object%20Reference) (Stimulus :type AI%20Stimulus%20Structure))
  (bind _asbp_third_person_character (Utilities|Casting|CastToBP_ThirdPersonCharacter Actor))
  (if (.bsuccessfullysensed Stimulus)
    (AI|Components|Blackboard|SetValueasObject (AI|GetBlackboard (Pawn|GetController)) (Utilities|Name|MakeLiteralName "PlayerRef") _asbp_third_person_character)
    (Utilities|Time|ClearandInvalidateTimerbyHandle (Variables|Default|GetLostVisionHandle))
    (else
      (bind _returnvalue (Utilities|Time|SetTimerbyEvent (delegate Custom|CustomEvent) 2.0))
      (Variables|Default|SetLostVisionHandle _returnvalue))))

(event Custom|CustomEvent
  (AI|Components|Blackboard|ClearValue (AI|GetBlackboard (Pawn|GetController)) (Utilities|Name|MakeLiteralName "PlayerRef")))

(event EventBeginPlay
  ;[0.1083 0.4844 0.01546 0.5] Setup a faire
  (bind _asaicontroller (Utilities|Casting|CastToAIController (Pawn|GetController)))
  (AI|RunBehaviorTree _asaicontroller "/Game/IA/BT_Test.BT_Test"))

(fn ConstructionScript)